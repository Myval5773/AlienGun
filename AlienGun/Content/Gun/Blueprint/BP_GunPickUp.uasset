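; BP_GunPickUp is a weapon pickup that reveals the third-person character's gun when that character overlaps its Box.
; The overlap casts to BP_ThirdPersonCharacter, makes its BPGun component visible and destroys the pickup.
; It then shows a WBP_TakeWeapon widget, with removal set after a Delay matching the FadeOut animation's end time.
; That Delay follows DestroyActor on the same actor, so the removal may never run.
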(event OnComponentBeginOverlap(Box)
  (params (OverlappedComponent :type Primitive%20Component%20Object%20Reference) (OtherActor :type Actor%20Object%20Reference) (OtherComp :type Primitive%20Component%20Object%20Reference) (OtherBodyIndex :type Integer) (bFromSweep :type Boolean) (SweepResult :type Hit%20Result%20Structure%20%28by%20ref%29))
  (bind _asbp_third_person_character (Utilities|Casting|CastToBP_ThirdPersonCharacter OtherActor))
  (Utilities|IsValid _asbp_third_person_character
    (:Is%20Valid
      (bind _output_get (Variables|Default|SetAs%20BP%20Third%20Person%20Character _asbp_third_person_character))
      (Rendering|SetVisibility (Variables|/Game/ThirdPerson/Blueprints/BP_ThirdPersonCharacter.BP_ThirdPersonCharacter_C|GetBP_Gun _output_get) true false)
      (Actor|DestroyActor)
      (bind _returnvalue (UserInterface|CreateWidget "/Game/ThirdPerson/Blueprints/WBP_TakeWeapon.WBP_TakeWeapon_C" (Game|GetPlayerController 0)))
      (UserInterface|Viewport|AddtoViewport _returnvalue 0)
      (Utilities|FlowControl|Delay (Class|WidgetAnimation|GetEndTime (Variables|/Game/ThirdPerson/Blueprints/WBP_TakeWeapon.WBP_TakeWeapon_C|GetFadeOut _returnvalue)))
      (Widget|RemovefromParent _returnvalue))))

(fn ConstructionScript)